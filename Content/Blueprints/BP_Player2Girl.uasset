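; Player character BP_Player2Girl with camera-relative movement, sprint, montage-flip double jump, dance, slap and item interaction.
; Slap plays a random montage and re-runs a hand-socket capsule trace every 0.01s until it hits a pawn or the montage ends, calling Hit on BP_AI.
; KeyInteract sends pickup and teleport interface messages to overlapping BP_RotatingItems; the line-trace interaction is disconnected.
; CanMove blocks movement during slap, pickup and dance.
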(event `self.ReceiveBeginPlay`
  (set `self.DefaultWalkSpeed` (`CharacterMovementComponent.MaxWalkSpeed` (`self.CharacterMovement`))))

(event `self.ReceiveTick`
  (params (DeltaSeconds :type "Float (single-precision)"))
  (bind _returnvalue (`self.K2_GetActorLocation`))
  (if (`NavMovementComponent.IsFalling` (`self.CharacterMovement`))
    (`KismetSystemLibrary.CapsuleTraceSingle` :`Start` _returnvalue :`End` _returnvalue :`TraceChannel` "TraceTypeQuery1" :`DrawDebugType` "ForOneFrame")))

(event `InputAxis|MoveForward`
  (params (AxisValue :type "Float (single-precision)"))
  ;[0 0 0 1 58] Movement Logic
  (if (`self.CanMove`)
    (`self.AddMovementInput` (`KismetMathLibrary.GetForwardVector` (`KismetMathLibrary.MakeRotator` 0.0 0.0 (.yaw (`self.GetControlRotation`)))) AxisValue)))

(event `InputAxis|MoveRight`
  (params (AxisValue :type "Float (single-precision)"))
  ;[0 0 0 1 58] Movement Logic
  (if (`self.CanMove`)
    (`self.AddMovementInput` (`KismetMathLibrary.GetRightVector` (`KismetMathLibrary.MakeRotator` 0.0 0.0 (.yaw (`self.GetControlRotation`)))) AxisValue)))

(event `InputAxis|LookUp`
  (params (AxisValue :type "Float (single-precision)"))
  ;[0 0 0 1 65] Look Logic
  (`self.AddControllerYawInput` AxisValue))

(event `InputAxis|Turn`
  (params (AxisValue :type "Float (single-precision)"))
  ;[0 0 0 1 65] Look Logic
  (`self.AddControllerPitchInput` AxisValue))

(event `InputAction|Jump`
  (params (Key :type "Key Structure"))
  (:`Pressed`
    (if (< (`self.JumpCount`) (`self.JumpMaxCount`))
      (if (`NavMovementComponent.IsFalling` (`self.CharacterMovement`))
        (`self.PlayAnimMontage` "/Game/Animations/Boy/JumpSet/doublejumpflip_Montage.doublejumpflip_Montage")
        (set `MovementComponent.Velocity` (`KismetMathLibrary.MakeVector` (.x (`self.GetVelocity`)) (.y (`self.GetVelocity`))) (`self.CharacterMovement`))
        (`self.LaunchCharacter` (+ (`self.GetVelocity`) (`KismetMathLibrary.MakeVector` 0.0 0.0 (`self.AirJumpVelocity`))) true true)
        (`/Engine/EditorBlueprintResources/StandardMacros.IncrementInt` (`self.JumpCount`))
        (else
          ;[1 1 1] ground jump
          (`self.Jump`)
          (`/Engine/EditorBlueprintResources/StandardMacros.IncrementInt` (`self.JumpCount`))))))
  (:`Released`
    (`self.StopJumping`)))

(event `InputAction|Sprint`
  (params (Key :type "Key Structure"))
  ;[0 0 0 1 74] Sprinting
  (:`Pressed`
    (set `CharacterMovementComponent.MaxWalkSpeed` (* (`self.SprintSpeedOffset`) (`self.DefaultWalkSpeed`)) (`self.CharacterMovement`)))
  (:`Released`
    (set `CharacterMovementComponent.MaxWalkSpeed` (`self.DefaultWalkSpeed`) (`self.CharacterMovement`))))

(event `self.OnLanded`
  (params (Hit :type "HitResult Structure (by ref)"))
  (set `self.JumpCount` 0))

(event `InputAction|Slap`
  (params (Key :type "Key Structure"))
  (bind _output (`|GetArrayItem` (`self.Slapping Anim Array`) (`KismetMathLibrary.RandomIntegerInRange` 0 2)))
  ;[0 0 0 1 82] slapping
  (:`Pressed`
    (set `self.CanMove` false)
    (if (and (not (`NavMovementComponent.IsFalling` (`self.CharacterMovement`))) (not (`self.IsSlapping`)))
      (set `self.IsSlapping` true)
      (set `self.LeftHand?` (`KismetStringLibrary.Contains` (`KismetSystemLibrary.GetDisplayName` _output) "Left"))
      (bind _returnvalue (`self.PlayAnimMontage` _output))
      (`|ExecutionSequence`
        (:`then_0`
          (`KismetSystemLibrary.Delay` _returnvalue)
          (set `self.IsSlapping` false)
          (set `self.CanMove` true))
        (:`then_1`
          (`self.PunchTrace`))))))

(event `PunchTrace`
  (bind _returnvalue (`SceneComponent.GetSocketLocation` (`self.Mesh`) (select `bool` (`self.LeftHand?`) :`false` "RightHand" :`true` "LeftHand" :!type "Name")))
  ;[0 0 0 1 82] slapping
  (if (`self.IsSlapping`)
    (bind (_outhit _returnvalue_2) (`KismetSystemLibrary.CapsuleTraceSingleForObjects` _returnvalue _returnvalue 22.0 22.0 (`|MakeArray` "ObjectTypeQuery3" :!type "EObjectTypeQuery Enum")))
    (if _returnvalue_2
      (bind _asbp_ai (cast `/Game/Blueprints/BP_AI` (`.HitActor` (`GameplayStatics.BreakHitResult` _outhit))))
      (`/Game/Blueprints/BP_AI.Hit` _asbp_ai)
      (else
        (`KismetSystemLibrary.Delay` 0.01)
        (`self.PunchTrace`)))))

(event `InputAction|Dance`
  (params (Key :type "Key Structure"))
  (:`Pressed`
    ;[0 0 0 1 122] dance
    (set `self.JumpMaxCount` 0)
    (set `self.CanMove` false)
    (`|PlayMontage` (`self.Mesh`) "/Game/Animations/Boy/Dance_Montage.Dance_Montage"))
  (:`Released`
    (set `self.JumpMaxCount` 2)
    (set `self.CanMove` true)
    (`SkeletalMeshComponent.SetAnimationMode` (`self.Mesh`) "AnimationBlueprint")))

(event `InputAction|KeyInteract`
  (params (Key :type "Key Structure"))
  ;[1 1 1] linetracing (pressed -> line trace)
)

(event `InputAction|KeyInteract`
  (params (Key :type "Key Structure"))
  ;[1 1 1] picking up
  (:`Pressed`
    (for _array_element (`self.GetOverlappingActors` "/Game/Blueprints/Picking_Up/BP_RotatingItem.BP_RotatingItem_C")
      (if (`KismetSystemLibrary.DoesImplementInterface` _array_element "/Game/Blueprints/BPI_Interactable.BPI_Interactable_C")
        (set `self.CanMove` false)
        (message `/Game/Blueprints/BPI_Interactable.PickUp` _array_element)
        (`|PlayMontage` (`self.Mesh`) "/Game/Animations/Boy/Pickup_Montage.Pickup_Montage" 2.0
          (:`then`
            (`KismetSystemLibrary.Delay` 1.5)
            (set `self.CanMove` true)))))))

(event `InputAction|KeyInteract`
  (params (Key :type "Key Structure"))
  ;[1 1 1] teleport
  (:`Pressed`
    (for _array_element (`self.GetOverlappingActors` "/Game/Blueprints/Picking_Up/BP_RotatingItem.BP_RotatingItem_C")
      (if (`KismetSystemLibrary.DoesImplementInterface` _array_element "/Game/Blueprints/BPI_Interactable.BPI_Interactable_C")
        (message `/Game/Blueprints/BPI_Interactable.Teleport` _array_element)))))

(fn `UserConstructionScript`)