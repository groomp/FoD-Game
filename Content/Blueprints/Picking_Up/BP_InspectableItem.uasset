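; Inspectable item actor with a configurable mesh that the player pulls up to the camera to examine and rotate.
; Sphere overlap toggles a prompt widget; Inspect attaches the item in front of the camera, disables collision and moves input from character to item.
; Left-mouse drag yaws it (MouseY adds zero pitch), while movement axes apply roll and yaw.
; The Inspect action restores the BeginPlay transform, collision and player input.
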(event `self.ReceiveBeginPlay`
  (set `self.Transform` (`self.GetTransform`)))

(event `self.Sphere.OnComponentBeginOverlap`
  (params (OverlappedComponent :type "PrimitiveComponent Object Reference") (OtherActor :type "Actor Object Reference") (OtherComp :type "PrimitiveComponent Object Reference") (OtherBodyIndex :type Integer) (bFromSweep :type Boolean) (SweepResult :type "HitResult Structure (by ref)"))
  ;[1 1 1] Check if we are close enough - do hud prompt
  (cast `/Game/Blueprints/BP_Player` OtherActor)
  (bind _returnvalue (`|CreateWidget` "/Game/Art/Prompts/InspectPrompt.InspectPrompt_C"))
  (`UserWidget.AddToViewport` _returnvalue 0))

(event `self.Sphere.OnComponentEndOverlap`
  (params (OverlappedComponent :type "PrimitiveComponent Object Reference") (OtherActor :type "Actor Object Reference") (OtherComp :type "PrimitiveComponent Object Reference") (OtherBodyIndex :type Integer))
  ;[1 1 1] Check if we are close enough - do hud prompt
  (cast `/Game/Blueprints/BP_Player` OtherActor)
  (`Widget.RemoveFromParent` (stale `self.Sphere.OnComponentBeginOverlap` _returnvalue)))

(event `/Game/Blueprints/BPI_Interactable.Inspect`
  (bind _returnvalue (`GameplayStatics.GetPlayerController` 0))
  (`KismetSystemLibrary.PrintString` "Inspecting...")
  (`self.SetActorEnableCollision` false)
  (`PrimitiveComponent.SetCollisionProfileName` (`self.Sphere`) "NoCollision" true)
  (`self.K2_AttachToComponent` (`PlayerCameraManager.TransformComponent` (`GameplayStatics.GetPlayerCameraManager` 0)) "None" "KeepWorld" "KeepWorld" "KeepWorld")
  (`KismetSystemLibrary.MoveComponentTo` (`self.DefaultSceneRoot`) (150.0 0.0 0.0))
  (`self.DisableInput` (`GameplayStatics.GetPlayerCharacter` 0) _returnvalue)
  (`self.EnableInput` _returnvalue))

(event `InputAction|Inspect`
  (params (Key :type "Key Structure"))
  (bind _returnvalue (`GameplayStatics.GetPlayerController` 0))
  (bind (_transform_location _transform_rotation) (`KismetMathLibrary.BreakTransform` (`self.Transform`)))
  ;[1 1 1] Reset back to original location and controls
  (:`Pressed`
    (`self.K2_DetachFromActor` "KeepWorld" "KeepWorld" "KeepWorld")
    (`KismetSystemLibrary.MoveComponentTo` (`self.DefaultSceneRoot`) _transform_location _transform_rotation)
    (`self.SetActorEnableCollision` true)
    (`PrimitiveComponent.SetCollisionProfileName` (`self.Sphere`) "OverlapAllDynamic" true)
    (`self.DisableInput` _returnvalue)
    (`self.EnableInput` (`GameplayStatics.GetPlayerCharacter` 0) _returnvalue)))

(event `Key|LeftMouseButton`
  (params (Key :type "Key Structure"))
  (:`Pressed`
    (set `self.CanRotate` true))
  (:`Released`
    (set `self.CanRotate` false)))

(event `InputAxisKey|MouseX`
  (params (AxisValue :type "Float (single-precision)"))
  (if (`self.CanRotate`)
    (`self.K2_SetActorRotation` (`KismetMathLibrary.ComposeRotators` (`self.K2_GetActorRotation`) (`KismetMathLibrary.MakeRotator` 0.0 0.0 (* AxisValue -2.0))))))

(event `InputAxisKey|MouseY`
  (params (AxisValue :type "Float (single-precision)"))
  (if (`self.CanRotate`)
    (`self.K2_SetActorRotation` (`KismetMathLibrary.ComposeRotators` (`self.K2_GetActorRotation`) (`KismetMathLibrary.MakeRotator` 0.0 (* 0.0 2.0))))))

(event `InputAxis|MoveForward`
  (params (AxisValue :type "Float (single-precision)"))
  (if (!= AxisValue 0.0)
    (`self.K2_SetActorRotation` (`KismetMathLibrary.ComposeRotators` (`self.K2_GetActorRotation`) (`KismetMathLibrary.MakeRotator` (* AxisValue -2.0))))))

(event `InputAxis|MoveRight`
  (params (AxisValue :type "Float (single-precision)"))
  (if (!= AxisValue 0.0)
    (`self.K2_SetActorRotation` (`KismetMathLibrary.ComposeRotators` (`self.K2_GetActorRotation`) (`KismetMathLibrary.MakeRotator` 0.0 0.0 (* AxisValue 2.0))))))

(fn `UserConstructionScript`
  (`StaticMeshComponent.SetStaticMesh` (`self.StaticMesh`) (`self.ItemModel`)))