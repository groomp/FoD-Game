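; Teleporter actor that moves the player character to a fixed world location when its Teleport event is called from outside this graph.
; A sphere overlap with BP_Player shows a TeleportPrompt widget and removes it on exit.
; The construction script applies the ItemModel mesh and places an arrow at TeleportLocation, but Teleport ignores that variable and uses hardcoded coordinates.
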(event `/Game/Blueprints/BPI_Interactable.Teleport`
  (`SceneComponent.K2_SetWorldTransform` (`Actor.RootComponent` (`GameplayStatics.GetPlayerCharacter` 0)) (`KismetMathLibrary.MakeTransform` (-2840.0 1140.0 2208.0)) false false))

(event `self.Sphere.OnComponentBeginOverlap`
  (params (OverlappedComponent :type "PrimitiveComponent Object Reference") (OtherActor :type "Actor Object Reference") (OtherComp :type "PrimitiveComponent Object Reference") (OtherBodyIndex :type Integer) (bFromSweep :type Boolean) (SweepResult :type "HitResult Structure (by ref)"))
  ;[1 1 1] Check if we are close enough - do hud prompt
  (cast `/Game/Blueprints/BP_Player` OtherActor)
  (bind _returnvalue (`|CreateWidget` "/Game/Art/Prompts/TeleportPrompt.TeleportPrompt_C"))
  (`UserWidget.AddToViewport` _returnvalue 0))

(event `self.Sphere.OnComponentEndOverlap`
  (params (OverlappedComponent :type "PrimitiveComponent Object Reference") (OtherActor :type "Actor Object Reference") (OtherComp :type "PrimitiveComponent Object Reference") (OtherBodyIndex :type Integer))
  ;[1 1 1] Check if we are close enough - do hud prompt
  (cast `/Game/Blueprints/BP_Player` OtherActor)
  (`Widget.RemoveFromParent` (stale `self.Sphere.OnComponentBeginOverlap` _returnvalue)))

(fn `UserConstructionScript`
  (`StaticMeshComponent.SetStaticMesh` (`self.StaticMesh`) (`self.ItemModel`))
  (`SceneComponent.K2_SetRelativeTransform` (`self.Arrow`) (`self.TeleportLocation`) false false))