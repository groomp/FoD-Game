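; BP_RotatingItem is a pickup item actor whose mesh is set from ItemModel in the construction script.
; A sphere overlap with BP_Player shows a PickupPrompt widget and removes it when the overlap ends.
; The PickUp event passes through a DoOnce to disable input, play a sound at the mesh, then destroy the actor after a short delay.
; No rotation logic appears in these graphs, and the EnableInput node is unconnected.
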(event `self.Sphere.OnComponentBeginOverlap`
  (params (OverlappedComponent :type "PrimitiveComponent Object Reference") (OtherActor :type "Actor Object Reference") (OtherComp :type "PrimitiveComponent Object Reference") (OtherBodyIndex :type Integer) (bFromSweep :type Boolean) (SweepResult :type "HitResult Structure (by ref)"))
  ;[1 1 1] Check if we are close enough - do hud prompt
  (cast `/Game/Blueprints/BP_Player` OtherActor)
  (bind _returnvalue (`|CreateWidget` "/Game/Art/Prompts/PickupPrompt.PickupPrompt_C"))
  (`UserWidget.AddToViewport` _returnvalue 0))

(event `self.Sphere.OnComponentEndOverlap`
  (params (OverlappedComponent :type "PrimitiveComponent Object Reference") (OtherActor :type "Actor Object Reference") (OtherComp :type "PrimitiveComponent Object Reference") (OtherBodyIndex :type Integer))
  ;[1 1 1] Check if we are close enough - do hud prompt
  (cast `/Game/Blueprints/BP_Player` OtherActor)
  (`Widget.RemoveFromParent` (stale `self.Sphere.OnComponentBeginOverlap` _returnvalue)))

(event `/Game/Blueprints/BPI_Interactable.PickUp`
  (`KismetSystemLibrary.PrintString` "event pick up called")
  ;[1 1 1] PICK UP / Destroy
  (`/Engine/EditorBlueprintResources/StandardMacros.DoOnce` false :!label _label
    (:`Completed`
      (`self.DisableInput` (`GameplayStatics.GetPlayerController` 0))
      (`KismetSystemLibrary.PrintString` "Picked up")
      (`GameplayStatics.PlaySoundAtLocation` "/Game/Sounds/Player/isee_Cue.isee_Cue" (`SceneComponent.K2_GetComponentLocation` (`self.StaticMesh`)) (struct) 1.0 1.0 0.0 null null null null)
      (`KismetSystemLibrary.Delay` 1.5)
      (`self.K2_DestroyActor`)
      (goto _label :!via `Reset`))))

(fn `UserConstructionScript`
  (`StaticMeshComponent.SetStaticMesh` (`self.StaticMesh`) (`self.ItemModel`)))