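; BP_HorrorAi is a horror AI actor that takes hits and is destroyed when its health runs out.
; It caches the player character on BeginPlay and checks its LeftHand flag to select a hit montage, though both options are the same montage.
; A DoOnce gates Hit while the slap sound and montage play, then subtracts Damage from Health after the montage's length, resetting only if health remains.
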(event `self.ReceiveBeginPlay`
  (bind _asbp_player_base (cast `/Game/Blueprints/BP_Player` (`GameplayStatics.GetPlayerCharacter` 0)))
  (set `self.CharacterRef` _asbp_player_base))

(event `Hit`
  (`/Engine/EditorBlueprintResources/StandardMacros.DoOnce` false :!label _label
    (:`Completed`
      (`GameplayStatics.PlaySoundAtLocation` "/Game/Sounds/Slap_Cue.Slap_Cue" (`self.K2_GetActorLocation`) (struct) 1.0 1.0 0.0 null null null null)
      (bind _returnvalue (`self.PlayAnimMontage` (select `bool` (`/Game/Blueprints/BP_Player.LeftHand?` (`self.CharacterRef`)) :`false` "/Game/Animations/Girl/gettinghit_Montage.gettinghit_Montage" :`true` "/Game/Animations/Girl/gettinghit_Montage.gettinghit_Montage" :!type "AnimMontage Object Reference")))
      (`KismetSystemLibrary.Delay` _returnvalue)
      (bind _output_get (set `self.Health` (- (`self.Health`) (`self.Damage`))))
      (if (<= _output_get 0)
        (`self.K2_DestroyActor`)
        (else
          (goto _label :!via `Reset`))))))

(fn `UserConstructionScript`)