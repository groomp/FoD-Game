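; Player character Blueprint with camera-relative movement, sprint, double jump with flip, glider, roll, dance and slap attacks.
; Slapping plays a random montage and re-runs a hand-socket capsule trace until it hits a BP_AI or the slap ends.
; Interact and Inspect inputs message overlapping items, teleporters and AI through BPI_Interactable.
; Musical pickups play successive notes, with a countdown timer resetting the sequence.
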(event `self.ReceiveBeginPlay`
  (set `self.camerarotation` true)
  (set `self.DefaultWalkSpeed` (`CharacterMovementComponent.MaxWalkSpeed` (`self.CharacterMovement`)))
  (bind _returnvalue (`|AddComponentByClass` "/Script/Engine.PostProcessComponent"))
  (setmembers `PostProcessSettings` :`StructRef` (`PostProcessComponent.Settings` _returnvalue) :`DepthOfFieldFstop` 0.8 :`DepthOfFieldSensorWidth` 80.0 :`DepthOfFieldFocalDistance` (`SpringArmComponent.TargetArmLength` (`self.SpringArm`))))

(event `self.ReceiveTick`
  (params (DeltaSeconds :type "Float (single-precision)"))
  (bind _returnvalue (`self.K2_GetActorLocation`))
  (if (`NavMovementComponent.IsFalling` (`self.CharacterMovement`))
    (`KismetSystemLibrary.CapsuleTraceSingle` :`Start` _returnvalue :`End` _returnvalue :`TraceChannel` "TraceTypeQuery1" :`DrawDebugType` "ForOneFrame")))

(event `HasPickedupMusical`
  (set `self.NumberOfMusicalPickups` (+ (`self.NumberOfMusicalPickups`) 1))
  (`self.CheckWhichMusicNote`)
  (if (> (`self.TimeleftMusical`) 0)
    (set `self.TimeleftMusical` 3)
    (bind _returnvalue (`KismetSystemLibrary.K2_SetTimer` null "Decrement" 1.0 true))
    (set `self.TimerHandle` _returnvalue)
    (else
      (set `self.NumberOfMusicalPickups` 1)
      (`KismetSystemLibrary.PrintString` "NOTES RESET")
      (set `self.TimeleftMusical` 3))))

(event `InputAxis|MoveForward`
  (params (AxisValue :type "Float (single-precision)"))
  ;[0 0 0 1 58] Movement Logic
  (if (`self.CanMove`)
    (`self.AddMovementInput` (`KismetMathLibrary.GetForwardVector` (`KismetMathLibrary.MakeRotator` 0.0 0.0 (.yaw (`self.GetControlRotation`)))) AxisValue)))

(event `InputAxis|MoveRight`
  (params (AxisValue :type "Float (single-precision)"))
  ;[0 0 0 1 58] Movement Logic
  (if (`self.CanMove`)
    (`self.AddMovementInput` (`KismetMathLibrary.GetRightVector` (`KismetMathLibrary.MakeRotator` 0.0 0.0 (.yaw (`self.GetControlRotation`)))) AxisValue)))

(event `InputAxis|LookUp`
  (params (AxisValue :type "Float (single-precision)"))
  ;[0 0 0 1 65] Look Logic
  (if (`self.camerarotation`)
    (`self.AddControllerYawInput` AxisValue)))

(event `InputAxis|Turn`
  (params (AxisValue :type "Float (single-precision)"))
  ;[0 0 0 1 65] Look Logic
  (if (`self.camerarotation`)
    (`self.AddControllerPitchInput` AxisValue)))

(event `InputAction|Jump`
  (params (Key :type "Key Structure"))
  ;[1 1 1] jumping
  (:`Pressed`
    (if (< (`self.JumpCount`) (`self.JumpMaxCount`))
      (if (`NavMovementComponent.IsFalling` (`self.CharacterMovement`))
        (`self.PlayAnimMontage` "/Game/Animations/Boy/JumpSet/doublejumpflip_Montage.doublejumpflip_Montage")
        (set `MovementComponent.Velocity` (`KismetMathLibrary.MakeVector` (.x (`self.GetVelocity`)) (.y (`self.GetVelocity`))) (`self.CharacterMovement`))
        (`self.LaunchCharacter` (+ (`self.GetVelocity`) (`KismetMathLibrary.MakeVector` 0.0 0.0 (`self.AirJumpVelocity`))) true true)
        (`/Engine/EditorBlueprintResources/StandardMacros.IncrementInt` (`self.JumpCount`))
        (else
          ;;[1 1 1] ground jump
          (`self.Jump`)
          (`/Engine/EditorBlueprintResources/StandardMacros.IncrementInt` (`self.JumpCount`))))))
  (:`Released`
    (`self.StopJumping`)))

(event `InputAction|Sprint`
  (params (Key :type "Key Structure"))
  ;[0 0 0 1 74] Sprinting
  (:`Pressed`
    (set `CharacterMovementComponent.MaxWalkSpeed` (* (`self.SprintSpeedOffset`) (`self.DefaultWalkSpeed`)) (`self.CharacterMovement`)))
  (:`Released`
    (set `CharacterMovementComponent.MaxWalkSpeed` (`self.DefaultWalkSpeed`) (`self.CharacterMovement`))))

(event `self.OnLanded`
  (params (Hit :type "HitResult Structure (by ref)"))
  ;[1 1 1] jumping
  (set `self.JumpCount` 0))

(event `InputAction|Slap`
  (params (Key :type "Key Structure"))
  (bind _returnvalue (`NavMovementComponent.IsFalling` (`self.CharacterMovement`)))
  (bind _output (`|GetArrayItem` (`self.Slapping Anim Array`) (`KismetMathLibrary.RandomIntegerInRange` 0 2)))
  ;[0 0 0 1 82] slapping
  (:`Pressed`
    (if (not _returnvalue)
      (set `self.CanMove` false)
      (if (and (not _returnvalue) (not (`self.IsSlapping`)))
        (set `self.IsSlapping` true)
        (set `self.LeftHand?` (`KismetStringLibrary.Contains` (`KismetSystemLibrary.GetDisplayName` _output) "Left"))
        (bind _returnvalue_2 (`self.PlayAnimMontage` _output))
        (`|ExecutionSequence`
          (:`then_0`
            (`KismetSystemLibrary.Delay` _returnvalue_2)
            (set `self.IsSlapping` false)
            (set `self.CanMove` true))
          (:`then_1`
            (`self.PunchTrace`)))))))

(event `PunchTrace`
  (bind _returnvalue (`SceneComponent.GetSocketLocation` (`self.Mesh`) (select `bool` (`self.LeftHand?`) :`false` "RightHand" :`true` "LeftHand" :!type "Name")))
  ;[0 0 0 1 82] slapping
  (if (`self.IsSlapping`)
    (bind (_outhit _returnvalue_2) (`KismetSystemLibrary.CapsuleTraceSingleForObjects` :`Start` _returnvalue :`End` _returnvalue :`Radius` 45.0 :`HalfHeight` 45.0 :`ObjectTypes` (`|MakeArray` "ObjectTypeQuery3" :!type "EObjectTypeQuery Enum") :`bTraceComplex` true :`DrawDebugType` "ForOneFrame"))
    (if _returnvalue_2
      (bind _asbp_ai (cast `/Game/Blueprints/BP_AI` (`.HitActor` (`GameplayStatics.BreakHitResult` _outhit))))
      (`/Game/Blueprints/BP_AI.Hit` _asbp_ai)
      (else
        (`KismetSystemLibrary.Delay` 0.01)
        (`self.PunchTrace`)))))

(event `InputAction|Dance`
  (params (Key :type "Key Structure"))
  (:`Pressed`
    ;[0 0 0 1 122] dance
    (set `self.JumpMaxCount` 0)
    (set `self.CanMove` false)
    (`|PlayMontage` (`self.Mesh`) "/Game/Animations/Boy/Dance_Montage.Dance_Montage"))
  (:`Released`
    (set `self.JumpMaxCount` 2)
    (set `self.CanMove` true)
    (`SkeletalMeshComponent.SetAnimationMode` (`self.Mesh`) "AnimationBlueprint")))

(event `InputAction|KeyInteract`
  (params (Key :type "Key Structure"))
  ;[1 1 1] linetracing (pressed -> line trace)
)

(event `InputAction|Roll`
  (params (Key :type "Key Structure"))
  (bind _charactermovement (`self.CharacterMovement`))
  ;[1 1 1] rolling
  (:`Pressed`
    (if (`NavMovementComponent.IsFalling` _charactermovement)
      _
      (elif (> (`KismetMathLibrary.VSize` (`MovementComponent.Velocity` _charactermovement)) 450.0)
        (`/Engine/EditorBlueprintResources/StandardMacros.DoOnce` false :!label _label
          (:`Completed`
            (`|PlayMontage` (`self.Mesh`) "/Game/Animations/Boy/Sprinting_Forward_Roll_Montage.Sprinting_Forward_Roll_Montage"
              (:`OnCompleted`
                (goto _label :!via `Reset`)))))))))

(event `InputAction|KeyInteract`
  (params (Key :type "Key Structure"))
  ;[1 1 1] picking up
  (:`Pressed`
    (for _array_element (`self.GetOverlappingActors` "/Game/Blueprints/Picking_Up/BP_RotatingItem.BP_RotatingItem_C")
      (if (`KismetSystemLibrary.DoesImplementInterface` _array_element "/Game/Blueprints/BPI_Interactable.BPI_Interactable_C")
        (set `self.CanMove` false)
        (message `/Game/Blueprints/BPI_Interactable.PickUp` _array_element)
        (`/Engine/EditorBlueprintResources/StandardMacros.DoOnce` false :!label _label_2
          (:`Completed`
            (`|PlayMontage` (`self.Mesh`) "/Game/Animations/Boy/Pickup_Montage.Pickup_Montage" 2.0
              (:`then`
                (`KismetSystemLibrary.Delay` 1.5)
                (set `self.CanMove` true)
                (goto _label_2 :!via `Reset`)))))))))

(event `InputAction|KeyInteract`
  (params (Key :type "Key Structure"))
  ;[1 1 1] teleport
  (:`Pressed`
    (for _array_element (`self.GetOverlappingActors` "/Game/Blueprints/Picking_Up/Teleporter.Teleporter_C")
      (if (`KismetSystemLibrary.DoesImplementInterface` _array_element "/Game/Blueprints/BPI_Interactable.BPI_Interactable_C")
        (message `/Game/Blueprints/BPI_Interactable.Teleport` _array_element)))))

(event `InputAction|KeyInteract`
  (params (Key :type "Key Structure"))
  ;[1 1 1] dialogue
  (:`Pressed`
    (for _array_element (`self.GetOverlappingActors` "/Game/Blueprints/BP_AI.BP_AI_C")
      (if (`KismetSystemLibrary.DoesImplementInterface` _array_element "/Game/Blueprints/BPI_Interactable.BPI_Interactable_C")
        (message `/Game/Blueprints/BPI_Interactable.IsSpeaking` _array_element null)
        (`KismetSystemLibrary.PrintString` "dialogue triggered!!!!")))))

(event `InputAction|Inspect`
  (params (Key :type "Key Structure"))
  ;[1 1 1] insepct
  (:`Pressed`
    (for _array_element (`self.GetOverlappingActors` "/Game/Blueprints/Picking_Up/BP_InspectableItem.BP_InspectableItem_C")
      (if (`KismetSystemLibrary.DoesImplementInterface` _array_element "/Game/Blueprints/BPI_Interactable.BPI_Interactable_C")
        (message `/Game/Blueprints/BPI_Interactable.Inspect` _array_element)))))

(event `InputAction|Gliding`
  (params (Key :type "Key Structure"))
  (:`Pressed`
    ;[1 1 1] gliding
    (if (`NavMovementComponent.IsFalling` (`self.CharacterMovement`))
      (if (`self.Gliding?`)
        (`self.DisableGlider`)
        (else
          (`self.EnableGlider`)))))
  (:`Released`
    (`self.DisableGlider`)))

(event `self.K2_OnMovementModeChanged`
  (params (PrevMovementMode :type "EMovementMode Enum" :default "MOVE_None") (NewMovementMode :type "EMovementMode Enum" :default "MOVE_None") (PrevCustomMode :type Byte) (NewCustomMode :type Byte))
  ;[1 1 1] gliding
  (if (`|EnumEquality` NewMovementMode "MOVE_Walking")
    (`self.DisableGlider`)))

(fn `CheckWhichMusicNote`
  (if (== (`self.NumberOfMusicalPickups`) 1)
    (`GameplayStatics.PlaySoundAtLocation` "/Game/Sounds/notes/F1_Cue.F1_Cue" (`SceneComponent.K2_GetComponentLocation` (`self.Mesh`)) (struct) 1.0 1.0 0.0 null null null null)
    (elif (== (`self.NumberOfMusicalPickups`) 2)
      (`GameplayStatics.PlaySoundAtLocation` "/Game/Sounds/notes/G_Cue.G_Cue" (`SceneComponent.K2_GetComponentLocation` (`self.Mesh`)) (struct) 1.0 1.0 0.0 null null null null)
      (elif (== (`self.NumberOfMusicalPickups`) 3)
        (`GameplayStatics.PlaySoundAtLocation` "/Game/Sounds/notes/A_Cue.A_Cue" (`SceneComponent.K2_GetComponentLocation` (`self.Mesh`)) (struct) 1.0 1.0 0.0 null null null null)
        (elif (== (`self.NumberOfMusicalPickups`) 4)
          (`GameplayStatics.PlaySoundAtLocation` "/Game/Sounds/notes/Bflatnote_Cue.Bflatnote_Cue" (`SceneComponent.K2_GetComponentLocation` (`self.Mesh`)) (struct) 1.0 1.0 0.0 null null null null)
          (elif (== (`self.NumberOfMusicalPickups`) 5)
            (`GameplayStatics.PlaySoundAtLocation` "/Game/Sounds/notes/Cnote_Cue.Cnote_Cue" (`SceneComponent.K2_GetComponentLocation` (`self.Mesh`)) (struct) 1.0 1.0 0.0 null null null null)
            (elif (== (`self.NumberOfMusicalPickups`) 6)
              (`GameplayStatics.PlaySoundAtLocation` "/Game/Sounds/notes/Dnote_Cue.Dnote_Cue" (`SceneComponent.K2_GetComponentLocation` (`self.Mesh`)) (struct) 1.0 1.0 0.0 null null null null)
              (elif (== (`self.NumberOfMusicalPickups`) 7)
                (`GameplayStatics.PlaySoundAtLocation` "/Game/Sounds/notes/Enote_Cue.Enote_Cue" (`SceneComponent.K2_GetComponentLocation` (`self.Mesh`)) (struct) 1.0 1.0 0.0 null null null null)
                (elif (== (`self.NumberOfMusicalPickups`) 8)
                  (`GameplayStatics.PlaySoundAtLocation` "/Game/Sounds/notes/Fchordnote_Cue.Fchordnote_Cue" (`SceneComponent.K2_GetComponentLocation` (`self.Mesh`)) (struct) 1.0 1.0 0.0 null null null null)
                  (elif (>= (`self.NumberOfMusicalPickups`) 9)
                    (`GameplayStatics.PlaySoundAtLocation` "/Game/Sounds/notes/Fchordnote_Cue.Fchordnote_Cue" (`SceneComponent.K2_GetComponentLocation` (`self.Mesh`)) (struct) 1.0 1.0 0.0 null null null null)))))))))))

(fn `Decrement`
  (bind _output_get (set `self.TimeleftMusical` (- (`self.TimeleftMusical`) 1)))
  (`KismetSystemLibrary.PrintString` (`KismetStringLibrary.Conv_IntToString` _output_get))
  (if (<= (`self.TimeleftMusical`) 0)
    (set `self.NumberOfMusicalPickups` 0)
    (`KismetSystemLibrary.K2_ClearAndInvalidateTimerHandle` (`self.TimerHandle`))))

(fn `DisableGlider`
  (set `self.Gliding?` false)
  (`SceneComponent.SetHiddenInGame` (`self.glider`) true false)
  (set `CharacterMovementComponent.GravityScale` 2.0 (`self.CharacterMovement`)))

(fn `EnableGlider`
  (bind _charactermovement (`self.CharacterMovement`))
  (bind (_velocity_x _velocity_y) (`KismetMathLibrary.BreakVector` (`MovementComponent.Velocity` _charactermovement)))
  (set `self.Gliding?` true)
  (`SceneComponent.SetHiddenInGame` (`self.glider`) false false)
  (set `MovementComponent.Velocity` (`KismetMathLibrary.MakeVector` (/ _velocity_x 6.0) (/ _velocity_y 6.0) -300.0) _charactermovement)
  (set `CharacterMovementComponent.GravityScale` 0.0 _charactermovement))

(fn `UserConstructionScript`)