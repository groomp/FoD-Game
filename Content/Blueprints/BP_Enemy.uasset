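; BP_Enemy is a jumpscare enemy that chases the player and sends them to the "horror" level on contact.
; When PawnSensing sees a pawn, it plays a jumpscare sound at its mesh and starts an AI MoveTo toward player 0.
; The IsSeeingPlayer flag gates the chase and is never cleared here.
; Overlapping BP_Player with the Levelteleporter component opens the horror level.
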(event `self.PawnSensing.OnSeePawn`
  (params (Pawn :type "Pawn Object Reference"))
  (set `self.isSeeingPlayer` true)
  (`GameplayStatics.PlaySoundAtLocation` "/Game/Sounds/misc/Jumpscare_Sound_Effect_Cue.Jumpscare_Sound_Effect_Cue" (`SceneComponent.K2_GetComponentLocation` (`self.Mesh`)) (struct) 1.0 1.0 0.0 null null null null)
  (`self.Follow Player`))

(event `Follow Player`
  (if (`self.isSeeingPlayer`)
    (`|AIMoveTo` self (0.0 0.0 0.0) (`GameplayStatics.GetPlayerCharacter` 0))))

(event `self.levelteleporter.OnComponentBeginOverlap`
  (params (OverlappedComponent :type "PrimitiveComponent Object Reference") (OtherActor :type "Actor Object Reference") (OtherComp :type "PrimitiveComponent Object Reference") (OtherBodyIndex :type Integer) (bFromSweep :type Boolean) (SweepResult :type "HitResult Structure (by ref)"))
  ;[1 1 1] send to scary level code
  (cast `/Game/Blueprints/BP_Player` OtherActor)
  (`GameplayStatics.OpenLevel` "horror"))

(fn `UserConstructionScript`)