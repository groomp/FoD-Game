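; BP_AI is an AI character that can be hit, loses health and dies.
; On BeginPlay it caches the player as BP_Player.
; Hit passes through a DoOnce gate, plays a slap sound and hit montage (the same montage for either player hand), then subtracts Damage after the montage's length.
; The gate resets while health remains; otherwise it plays death sound and animation, then destroys the actor after a delay.
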(event `self.ReceiveBeginPlay`
  (bind _asbp_player (cast `/Game/Blueprints/BP_Player` (`GameplayStatics.GetPlayerCharacter` 0)))
  (set `self.CharacterRef` _asbp_player))

(event `Hit`
  ;[1 1 1] getting hit
  (`/Engine/EditorBlueprintResources/StandardMacros.DoOnce` false :!label _label
    (:`Completed`
      (`GameplayStatics.PlaySoundAtLocation` "/Game/Sounds/Slap_Cue.Slap_Cue" (`self.K2_GetActorLocation`) (struct) 1.0 1.0 0.0 null null null null)
      (bind _returnvalue (`self.PlayAnimMontage` (select `bool` (`/Game/Blueprints/BP_Player.LeftHand?` (`self.CharacterRef`)) :`false` "/Game/Animations/Girl/gettinghit_Montage.gettinghit_Montage" :`true` "/Game/Animations/Girl/gettinghit_Montage.gettinghit_Montage" :!type "AnimMontage Object Reference")))
      (`KismetSystemLibrary.Delay` _returnvalue)
      (bind _output_get (set `self.Health` (- (`self.Health`) (`self.Damage`))))
      (if (<= _output_get 0)
        (`GameplayStatics.PlaySoundAtLocation` "/Game/Sounds/aaaa_im_dying_Cue.aaaa_im_dying_Cue" (`self.K2_GetActorLocation`) (struct) 1.0 1.0 0.0 null null null null)
        (`SkeletalMeshComponent.PlayAnimation` (`self.Mesh`) "/Game/Animations/Girl/Falling_Back_Death.Falling_Back_Death" false)
        (`KismetSystemLibrary.Delay` 4.0)
        (`self.K2_DestroyActor`)
        (else
          (goto _label :!via `Reset`))))))

(fn `UserConstructionScript`)